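; Game mode for a Pac-Man style game that sets starting lives and score, plays sounds and spawns the ghosts.
; SpawnGhosts releases Blinky, Pinky, Inky and Clyde on staggered delays, each at the GhostSpawnPoint.
; OnReset destroys the player character, waits, respawns and possesses a new one at the PlayerStart, then restarts the ghost sequence without removing existing ghosts.
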(event Custom|SpawnGhosts
  ;[1 1 1] SpawnGhosts
  (Utilities|FlowControl|Delay 3.0)
  (CallFunction|SpawnGhost "/Game/Blueprints/AI/Blinky/Blinky.Blinky_C")
  (Utilities|FlowControl|Delay 1e+01)
  (CallFunction|SpawnGhost "/Game/Blueprints/AI/Pinky/Pinky.Pinky_C")
  (Utilities|FlowControl|Delay 1e+01)
  (CallFunction|SpawnGhost "/Game/Blueprints/AI/Inky/Inky.Inky_C")
  (Utilities|FlowControl|Delay 1e+01)
  (CallFunction|SpawnGhost "/Game/Blueprints/AI/Clyde/Clyde.Clyde_C"))

(event EventBeginPlay
  (Variables|Default|SetLives 3)
  (Variables|Default|SetScore 0)
  (CallFunction|SpawnGhosts)
  (Audio|PlaySound2D "/Game/Audio/PacManChomp.PacManChomp" 1.0 1.0 0.0 0 0)
  (Audio|PlaySound2D "/Game/Audio/BackgroundAmbientMusic.BackgroundAmbientMusic" 1.0 1.0 0.0 0 0)
  (Audio|PlaySound2D "/Game/Audio/BackgroundMusicDeath.BackgroundMusicDeath" 1.0 1.0 0.0 0 0))

(event EventTick
  (params (DeltaSeconds :type Float%20%28single-precision%29)))

(event EventOnReset
  (bind _returnvalue (Actor|GetActorOfClass "/Game/Blueprints/PlayerCharacer_BP.PlayerCharacer_BP_C"))
  (Utilities|IsValid _returnvalue
    (:Is%20Valid
      (Actor|DestroyActor _returnvalue))
    (:Is%20Not%20Valid
      _))
  (Utilities|FlowControl|Delay 3.0)
  (bind _returnvalue_2 (Actor|GetActorOfClass "/Script/Engine.PlayerStart"))
  (bind _returnvalue_3 (Game|SpawnActorfromClass "/Game/Blueprints/PlayerCharacer_BP.PlayerCharacer_BP_C" (Transformation|GetActorTransform _returnvalue_2) "AlwaysSpawn" 0 0))
  (Pawn|Possess (Game|GetPlayerController 0) _returnvalue_3)
  (Variables|/Script/PacMan1stPersHorror.PlayerCharacter|SetIsPlayerDead _returnvalue_3 false)
  (CallFunction|SpawnGhosts))

(fn ConstructionScript)

(fn SpawnGhost
  (params (Class :type Actor%20Class%20Reference))
  (bind _returnvalue (Actor|GetActorOfClass "/Game/Blueprints/AI/GhostSpawnPoint.GhostSpawnPoint_C"))
  (Game|SpawnActorfromClass Class (Transformation|GetActorTransform _returnvalue) "AlwaysSpawn" 0 0))