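; Behavior tree task that steps an AI pawn one tile at a time toward a target actor on the TileGen_BP tile map.
; It asks the tile generator for the tile closest to the target, passing the previous tile from the blackboard, then stores the pawn's current tile as the new previous one.
; The pawn moves there with SimpleMoveToLocation, and the task finishes successfully on the controller's move-completed event, whatever the result.
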(event Custom|ReceiveMoveCompleted_Event_0
  (params (RequestID :type AI%20Request%20ID%20Structure) (Result :type EPathFollowingResult%20Enum :default "Success"))
  (AI|BehaviorTree|FinishExecute true))

(event EventReceiveExecuteAI
  (params (OwnerController :type AI%20Controller%20Object%20Reference) (ControlledPawn :type Pawn%20Object%20Reference))
  (bind _returnvalue (AI|GetBlackboard OwnerController))
  (bind _returnvalue_2 (Transformation|GetActorLocation ControlledPawn))
  (bind _prevtilename (Variables|Default|GetPrevTileName))
  (Utilities|FlowControl|Sequence
    (:then_0
      ;[1 1 1] Finding next tile to move to
      (bind _returnvalue_3 (Actor|GetActorOfClass (Variables|Default|GetTargetActor)))
      (bind _returnvalue_4 (Actor|GetActorOfClass "/Game/Blueprints/AI/TileGen_BP.TileGen_BP_C"))
      (bind _returnvalue_5 (Class|TileGenerator|GetClosestTiletoTarget _returnvalue_4 _returnvalue_2 (Transformation|GetActorLocation _returnvalue_3) (Class|BlackboardComponent|GetValueasInt _returnvalue _prevtilename)))
      (Utilities|FlowControl|Sequence
        (:then_0
          ;[1 1 1] Setting CurrentTile as PrevTile
          (bind _returnvalue_6 (Class|TileGenerator|GetTilefromCoordinates _returnvalue_4 _returnvalue_2))
          (Class|BlackboardComponent|SetValueasInt _returnvalue _prevtilename _returnvalue_6))
        (:then_1
          (bind _returnvalue_7 (Class|TileGenerator|GetCoordinatesfromTile _returnvalue_4 _returnvalue_5))
          (AI|Navigation|SimpleMovetoLocation OwnerController _returnvalue_7))))
    (:then_1
      (EventDispatchers|AssignReceiveMoveCompleted OwnerController (delegate Custom|ReceiveMoveCompleted_Event_0)))))