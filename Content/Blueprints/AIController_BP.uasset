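; AI controller that runs BlinkBehaviourTree and keeps its Blackboard updated with the player's position on a generated tile map.
; On BeginPlay it stores the player character and the level's TileGen_BP in the Blackboard, then starts the tree.
; Each Tick it converts the player's location to a tile and back to coordinates through TileGen_BP, writing the result to PlayerLocation.
; The Tick also prints each conversion step for debugging.
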(event EventBeginPlay
  (bind _blackboardcomponent (Class|AIController|UseBlackboard "/Game/Blueprints/NewBlackboardData_BP.NewBlackboardData_BP"))
  (AI|Components|Blackboard|SetValueasObject _blackboardcomponent (Variables|Default|GetPlayerKey) (Game|GetPlayerCharacter 0))
  (bind _returnvalue (Actor|GetActorOfClass "/Game/Blueprints/TileGen_BP.TileGen_BP_C"))
  (AI|Components|Blackboard|SetValueasObject _blackboardcomponent (Variables|Default|GetTileGenerator) _returnvalue)
  (AI|RunBehaviorTree "/Game/Blueprints/BlinkBehaviourTree.BlinkBehaviourTree"))

(event EventTick
  (params (DeltaSeconds :type Float%20%28single-precision%29))
  (bind _returnvalue (Game|GetPlayerCharacter 0))
  (bind _returnvalue_2 (Transformation|GetActorLocation _returnvalue))
  (bind _blackboardcomponent (Class|AIController|UseBlackboard "/Game/Blueprints/NewBlackboardData_BP.NewBlackboardData_BP"))
  (bind _astile_gen_bp (Utilities|Casting|CastToTileGen_BP (AI|Components|Blackboard|GetValueasObject _blackboardcomponent (Variables|Default|GetTileGenerator))))
  (bind _returnvalue_3 (Class|TileGenerator|GetTilefromCoordinates _astile_gen_bp _returnvalue_2))
  (Development|PrintString (Utilities|String|ToString(Vector) _returnvalue_2))
  (Development|PrintString (Utilities|String|ToString(Integer) _returnvalue_3))
  (bind _returnvalue_4 (Class|TileGenerator|GetCoordinatesfromTile _astile_gen_bp (Math|Conversions|ToInteger(Byte) (Utilities|String|ToString(Integer) _returnvalue_3))))
  (Development|PrintString (Utilities|String|ToString(Vector) _returnvalue_4))
  (AI|Components|Blackboard|SetValueasVector _blackboardcomponent (Variables|Default|GetPlayerLocation) _returnvalue_4))

(fn ConstructionScript)