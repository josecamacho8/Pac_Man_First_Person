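; Player character Blueprint for what appears to be a Pac-Man-style game, tracking grid position, pickups and death.
; Tick looks up the TileGenerator and converts the actor's location to a tile, shifting CurrentTile into PrevTile on change.
; Overlaps either consume a powerup for a timed PlayerPowerup state or add score to the game mode.
; Any other overlap plays a ghost-eating sound while powered up, otherwise flags the player dead.
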(event EventBeginPlay
  (Variables|Default|SetPrevTile 0))

(event EventTick
  (params (DeltaSeconds :type Float%20%28single-precision%29))
  (bind _returnvalue (Actor|GetActorOfClass "/Script/PacMan1stPersHorror.TileGenerator"))
  (bind _returnvalue_2 (Class|TileGenerator|GetTilefromCoordinates _returnvalue (Transformation|GetActorLocation)))
  (if (not (== (Class|KismetMathLibrary|ToInt64(Integer) _returnvalue_2) (Class|KismetMathLibrary|ToInt64(Integer) (Variables|Default|GetCurrentTile))))
    (Variables|Default|SetPrevTile (Variables|Default|GetCurrentTile))
    (Variables|Default|SetCurrentTile _returnvalue_2)))

(event Collision|EventActorBeginOverlap
  (params (OtherActor :type Actor%20Object%20Reference))
  (bind _aspowerup_blueprint (Utilities|Casting|CastToPowerup_Blueprint OtherActor)
    (:then
      ;[1 1 1] Overlap With Powerup
      (Variables|Default|SetPlayerPowerup true)
      (Actor|DestroyActor _aspowerup_blueprint)
      (Utilities|FlowControl|Delay 5.0)
      (Variables|Default|SetPlayerPowerup false))
    (:CastFailed
      (Utilities|Casting|CastToScorePickup_Blueprint OtherActor
        (:then
          (bind _asdefault_game_mode_base (Utilities|Casting|CastToDefaultGameModeBase (Game|GetGameMode)))
          (Variables|/Game/Blueprints/DefaultGameModeBase.DefaultGameModeBase_C|SetScore _asdefault_game_mode_base (+ (Variables|/Game/Blueprints/DefaultGameModeBase.DefaultGameModeBase_C|GetScore _asdefault_game_mode_base) 100)))
        (:CastFailed
          (if (Variables|Default|GetPlayerPowerup)
            (Audio|PlaySound2D "/Game/Audio/Cue_EatingGhost.Cue_EatingGhost" 1.0 1.0 0.0 0 0)
            (else
              (Variables|Default|SetIsPlayerDead true))))))))

(fn ConstructionScript)